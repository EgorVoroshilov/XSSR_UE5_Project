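; BP_GridManager owns the grid actors used by the survival kit's building system, one per build part type such as foundation, wall, stairs or roof.
; On BeginPlay it loops the build type enum, spawns each type's valid grid class and stores it in a typed variable.
; SelectGridActor maps a type to its actor, which GetAllGrids uses to list them and DeleteGrid uses to route component removal to the matching grid.
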(fn `CreateGridActors`
  (locals (GridTypeL :type "/Game/SurvivalGameKitV2/Blueprints/Other/Enum/E_BuildType Enum") (NewGrid :type "/Game/SurvivalGameKitV2/Blueprints/Grids/BP_MasterGrid Object Reference"))
  ;[1 1 1] Spawns a grid actor for each build part type
  (bind _enumvalue (foreach `/Game/SurvivalGameKitV2/Blueprints/Other/Enum/E_BuildType` true)
    (:`LoopBody`
      (bind _output_get (set `local.GridTypeL` _enumvalue))
      (bind _grid (`/Game/SurvivalGameKitV2/Blueprints/Other/Interfaces/BP_SGKFunctions.SGK GridClasses` _output_get))
      (if (`KismetSystemLibrary.IsValidClass` _grid)
        (bind _returnvalue (`|SpawnActorFromClass` _grid (`KismetMathLibrary.MakeTransform` (0.0 0.0 0.0)) "AlwaysSpawn" "OverrideRootScale" null null))
        (set `local.NewGrid` _returnvalue)
        (switch `/Game/SurvivalGameKitV2/Blueprints/Other/Enum/E_BuildType` (`local.GridTypeL`)
          (:`NewEnumerator1`
            (set `self.FoundationGrid` (`local.NewGrid`)))
          (:`NewEnumerator2`
            (set `self.WallGrid` (`local.NewGrid`)))
          (:`NewEnumerator4`
            (set `self.TriangleFoundationGrid` (`local.NewGrid`)))
          (:`NewEnumerator5`
            (set `self.FloorGrid` (`local.NewGrid`)))
          (:`NewEnumerator6`
            (set `self.TriangleFloorGrid` (`local.NewGrid`)))
          (:`NewEnumerator7`
            (set `self.StairsGrid` (`local.NewGrid`)))
          (:`NewEnumerator8`
            (set `self.DoorGrid` (`local.NewGrid`)))
          (:`NewEnumerator9`
            (set `self.WindowGrid` (`local.NewGrid`)))
          (:`NewEnumerator11`
            (set `self.LockGrid` (`local.NewGrid`)))
          (:`NewEnumerator12`
            (set `self.RoofGrid` (`local.NewGrid`)))
          (:`NewEnumerator13`
            (set `self.DoubleDoorGrid` (`local.NewGrid`))))))))

(fn `DeleteGrid`
  (params (Grid :type "BoxComponent Object Reference"))
  ;[1 1 1] Delete the input grid component from the grid actor
  (`/Engine/EditorBlueprintResources/StandardMacros.IsValid` Grid
    (:`Is Valid`
      (bind _asbp_master_grid (cast `/Game/SurvivalGameKitV2/Blueprints/Grids/BP_MasterGrid` (`ActorComponent.GetOwner` Grid)))
      (bind _grid (`self.SelectGridActor` (`/Game/SurvivalGameKitV2/Blueprints/Grids/BP_MasterGrid.GridType` _asbp_master_grid)))
      (`/Engine/EditorBlueprintResources/StandardMacros.IsValid` _grid
        (:`Is Valid`
          (`/Game/SurvivalGameKitV2/Blueprints/Grids/BP_MasterGrid.DeleteGrid` _grid (`local.Grid`)))))))

(fn `GetAllGrids`
  (returns (AllGrids :type "Array of /Game/SurvivalGameKitV2/Blueprints/Grids/BP_MasterGrid Object Reference"))
  (locals (AllGridsL :type "Array of /Game/SurvivalGameKitV2/Blueprints/Grids/BP_MasterGrid Object Reference"))
  ;[1 1 1] Return an array of all grid actors
  (bind _enumvalue (foreach `/Game/SurvivalGameKitV2/Blueprints/Other/Enum/E_BuildType` true)
    (:`LoopBody`
      (bind _grid (`self.SelectGridActor` _enumvalue))
      (`KismetArrayLibrary.Array_Add` (`local.AllGridsL`) _grid))
    (:`then`
      (return (`local.AllGridsL`)))))

(fn `SelectGridActor`
  (params (GridType :type "/Game/SurvivalGameKitV2/Blueprints/Other/Enum/E_BuildType Enum" :default "NewEnumerator0"))
  (returns (Grid :type "/Game/SurvivalGameKitV2/Blueprints/Grids/BP_MasterGrid Object Reference"))
  ;[1 1 1] Return the grid actor for the grid type
  (return (select `/Game/SurvivalGameKitV2/Blueprints/Other/Enum/E_BuildType` GridType :`NewEnumerator1` (`self.FoundationGrid`) :`NewEnumerator2` (`self.WallGrid`) :`NewEnumerator4` (`self.TriangleFoundationGrid`) :`NewEnumerator5` (`self.FloorGrid`) :`NewEnumerator6` (`self.TriangleFloorGrid`) :`NewEnumerator7` (`self.StairsGrid`) :`NewEnumerator8` (`self.DoorGrid`) :`NewEnumerator9` (`self.WindowGrid`) :`NewEnumerator11` (`self.LockGrid`) :`NewEnumerator12` (`self.RoofGrid`) :`NewEnumerator13` (`self.DoubleDoorGrid`))))

(fn `UserConstructionScript`)