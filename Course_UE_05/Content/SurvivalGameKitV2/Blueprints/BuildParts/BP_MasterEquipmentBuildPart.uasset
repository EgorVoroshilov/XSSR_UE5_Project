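; Master build part for placeable containers that hold an equipment inventory, searched through the SGK interaction interface.
; BeginPlay initializes the equipment inventory component and its save system.
; Interacting registers the player as a user and opens the external equipment inventory via server calls, and ending interaction removes that user.
; Loading restores EquipmentSaveData by index from the current level's save, while SaveExtraData calls PrepareCookingSaveData rather than an equipment-specific function.
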(fn `SaveExtraData`
  (params (SaveGame :type "/Game/SurvivalGameKitV2/Blueprints/Saving/BP_SGKSaveGame Object Reference") (LevelSaveData :type "/Game/SurvivalGameKitV2/Blueprints/Other/Structs/S_LevelSaveData Structure"))
  (returns (ExtraDataIndex :type Integer) (NewLevelSaveData :type "/Game/SurvivalGameKitV2/Blueprints/Other/Structs/S_LevelSaveData Structure"))
  (bind (_extradataindex _newlevelsavedata) (`/Game/SurvivalGameKitV2/Blueprints/Saving/BP_SGKSaveGame.PrepareCookingSaveData` SaveGame null LevelSaveData))
  (return _extradataindex _newlevelsavedata))

(fn `SGK AllowInteraction`
  (returns (AllowInteraction :type Boolean))
  (`parent.SGK AllowInteraction`)
  (return true))

(fn `SGK CharacterCamera`
  (params (CameraType :type "/Game/SurvivalGameKitV2/Blueprints/Other/Enum/E_CameraType Enum" :default "NewEnumerator0"))
  (returns (CurrentCamera :type "CameraComponent Object Reference") (CurrentSpringArm :type "SpringArmComponent Object Reference"))
  (return null null))

(fn `SGK CharacterSockets`
  (params (Sockets :type "/Game/SurvivalGameKitV2/Blueprints/Other/Enum/E_Sockets Enum" :default "NewEnumerator0"))
  (returns (Component :type "SceneComponent Object Reference"))
  (return null))

(fn `SGK EndInteraction`
  (params (PlayerInventory :type "/Game/SurvivalGameKitV2/Components/BP_PlayerInventory Object Reference"))
  (returns (ReturnValue :type Boolean))
  (bind _bp_equipmentinventory (`self.BP_EquipmentInventory`))
  (`/Engine/EditorBlueprintResources/StandardMacros.IsValid` _bp_equipmentinventory
    (:`Is Valid`
      (`/Game/SurvivalGameKitV2/Components/BP_EquipmentInventory.ServerRemoveUserToEquipmentItems` _bp_equipmentinventory (`local.PlayerInventory`) false)
      (return false))))

(fn `SGK GetMesh`
  (params (MeshType :type "/Game/SurvivalGameKitV2/Blueprints/Other/Enum/E_BodyMesh Enum" :default "NewEnumerator0"))
  (returns (Mesh :type "PrimitiveComponent Object Reference"))
  (return (`self.SkeletalMesh`)))

(fn `SGK Interact`
  (params (PlayerInventory :type "/Game/SurvivalGameKitV2/Components/BP_PlayerInventory Object Reference") (Action :type "/Game/SurvivalGameKitV2/Blueprints/Other/Enum/E_WorldActions Enum" :default "NewEnumerator0"))
  (returns (ReturnValue :type Boolean))
  (bind _bp_equipmentinventory (`self.BP_EquipmentInventory`))
  ;[1 1 1] On interact add using play and open equipment inv
  (`/Game/SurvivalGameKitV2/Components/BP_EquipmentInventory.ServerAddUserToEquipmentItems` _bp_equipmentinventory PlayerInventory)
  (`/Game/SurvivalGameKitV2/Components/BP_PlayerInventory.ServerOpenExtEquipmentInv` PlayerInventory _bp_equipmentinventory)
  (return true))

(fn `SGK InteractName`
  (returns (InteractName :type Text))
  (`parent.SGK InteractName`)
  (return "SEARCH CONTAINER"))

(fn `SGK LeanValues`
  (returns (`Lean Alpha` :type "Float (double-precision)") (TargetCamera :type "Float (double-precision)"))
  (return 0.0 0.0))

(fn `SGK LookAtRotation`
  (returns (LookAtRotation :type "Vector2D Structure"))
  (return (0.0 0.0)))

(fn `SGK PossibleActions`
  (params (PlayerInventory :type "/Game/SurvivalGameKitV2/Components/BP_PlayerInventory Object Reference"))
  (returns (ActionsFound :type Boolean) (PossibleActions :type "Array of /Game/SurvivalGameKitV2/Blueprints/Other/Structs/S_WorldAction Structure"))
  (return true (`|MakeArray` (make `/Game/SurvivalGameKitV2/Blueprints/Other/Structs/S_WorldAction` "NewEnumerator3" "OPEN"))))

(fn `UserConstructionScript`
  (`parent.UserConstructionScript`))