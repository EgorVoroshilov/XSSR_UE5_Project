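; Wooden chest furniture build part that shows an open or closed lid by swapping its static mesh.
; The turned-on effect event sets the open mesh and flushes net dormancy, but does nothing when turned off.
; Closing happens in the end-interaction override, which calls the parent, restores the closed mesh and returns false.
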(fn `SGK EndInteraction`
  (params (PlayerInventory :type "/Game/SurvivalGameKitV2/Components/BP_PlayerInventory Object Reference"))
  (returns (ReturnValue :type Boolean))
  ;[1 1 1] Set mesh to closed when player ends interaction
  (`parent.SGK EndInteraction` PlayerInventory)
  (`StaticMeshComponent.SetStaticMesh` (`self.StaticMesh`) "/Game/SurvivalGameKitV2/Meshes/Static/SM_Chest_Closed.SM_Chest_Closed")
  (return false))

(fn `UserConstructionScript`
  (`parent.UserConstructionScript`))