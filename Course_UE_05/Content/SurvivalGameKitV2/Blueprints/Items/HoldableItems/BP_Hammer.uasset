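; Holdable hammer item that serves as the player's building tool and melee weapon.
; Holding secondary action sets the build mode and opens a radial menu through the player's building component.
; Primary action selects the hovered segment when that menu exists, briefly setting a server-side flag that blocks the melee swing, which is also suppressed in build mode.
; A build-controls overlay widget shows while the hammer is held.
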(event `ServerBlockSwing`
  (params (Block :type Boolean))
  ;[1 1 1] Server set block swing
  (set `self.BlockSwing` Block))

(event `self.SGK ServerPrimaryAction`
  (params (KeyDown :type Boolean))
  ;[1 1 1] On server primary action check if build menu is open, if not allow melee swing
  (if KeyDown
    (if (`/Game/SurvivalGameKitV2/Components/BP_PlayerInventory.BuildMode` (`self.PlayerInventory`))
      _
      (elif (not (`self.BlockSwing`))
        (`parent.SGK ServerPrimaryAction` KeyDown)))
    (else
      (`parent.SGK ServerPrimaryAction` false))))

(event `self.SGK ClientPrimaryAction`
  (params (KeyDown :type Boolean))
  ;[1 1 1] On client primary action check if build menu is open and if it is select the mouse over segment and block melee attack
  (if KeyDown
    (bind _playerhud (`/Game/SurvivalGameKitV2/Components/BP_PlayerInventory.PlayerHUD` (`self.PlayerInventory`))
      (:`then`
        (bind _radialmenu (`/Game/SurvivalGameKitV2/Blueprints/Widgets/BP_InventoryHUD.RadialMenu` _playerhud)
          (:`then`
            (`/Game/SurvivalGameKitV2/Blueprints/Widgets/BP_MasterRadialMenu.SelectSegment` _radialmenu)
            (`self.ServerBlockSwing` true)
            (`/Game/SurvivalGameKitV2/Components/BP_PlayerBuildingComponent.SelectBuildMode` (`/Game/SurvivalGameKitV2/Components/BP_PlayerInventory.PlayerBuildingComponent` (`self.PlayerInventory`)) "NewEnumerator3")
            (`KismetSystemLibrary.RetriggerableDelay` 0.2)
            (`self.ServerBlockSwing` false))
          (:`else`
            (`parent.SGK ClientPrimaryAction` KeyDown))))
      (:`else`))))

(event `self.SGK ClientSecondaryAction`
  (params (KeyDown :type Boolean))
  (bind _playerbuildingcomponent (`/Game/SurvivalGameKitV2/Components/BP_PlayerInventory.PlayerBuildingComponent` (`self.PlayerInventory`)))
  ;[1 1 1] On client secondary action open build radial menu on key down and close on key up
  (`/Game/SurvivalGameKitV2/Components/BP_PlayerBuildingComponent.SelectBuildMode` _playerbuildingcomponent (select `bool` KeyDown :`false` "NewEnumerator3" :`true` "NewEnumerator4" :!type "/Game/SurvivalGameKitV2/Blueprints/Other/Enum/E_BuildingMode Enum"))
  (`/Game/SurvivalGameKitV2/Components/BP_PlayerBuildingComponent.BuildTrace` _playerbuildingcomponent)
  (`self.ToggleBuildMenu` KeyDown)
  (`parent.SGK ClientSecondaryAction` KeyDown))

(event `self.SGK ResetHoldable`
  ;[1 1 1] Resets the holdable to clear build menu and unblock swing
  (`/Game/SurvivalGameKitV2/Components/BP_PlayerBuildingComponent.ClientRemoveMenu` (`/Game/SurvivalGameKitV2/Components/BP_PlayerInventory.PlayerBuildingComponent` (`self.PlayerInventory`)))
  (`self.ServerBlockSwing` false)
  (`self.ClientRemoveOverlayWidget`)
  (`parent.SGK ResetHoldable`))

(event `self.SGK NewHeld`
  (params (Held :type Boolean))
  ;[1 1 1] Add build controls widget overlay when held and hide when unheld
  (`parent.SGK NewHeld` Held)
  (if Held
    (`self.ClientAddOverlayWidget`)
    (else
      (`self.ClientRemoveOverlayWidget`))))

(event `ClientAddOverlayWidget`
  ;[1 1 1] Create build controls widget and add to screen
  (bind _playerinventory (`self.PlayerInventory`)
    (:`then`
      (bind _asplayer_controller (cast `PlayerController` (`Pawn.GetController` (`/Game/SurvivalGameKitV2/Components/BP_EquipmentInventory.OwningCharacter` _playerinventory)) :!pure true))
      (`/Engine/EditorBlueprintResources/StandardMacros.IsValid` _asplayer_controller
        (:`Is Valid`
          (bind _returnvalue (`|CreateWidget` "/Game/SurvivalGameKitV2/Blueprints/Widgets/BP_HammerOverlay.BP_HammerOverlay_C" _asplayer_controller))
          (set `self.OverlayWidget` _returnvalue)
          (`UserWidget.AddToViewport` _returnvalue -1))))
    (:`else`)))

(event `self.ReceiveDestroyed`
  ;[1 1 1] On destroy remove build controls widget
  (bind _overlaywidget (`self.OverlayWidget`)
    (:`then`
      (`Widget.RemoveFromParent` _overlaywidget))
    (:`else`)))

(event `ClientRemoveOverlayWidget`
  ;[1 1 1] Client removes overlay widget
  (bind _overlaywidget (`self.OverlayWidget`)
    (:`then`
      (`Widget.RemoveFromParent` _overlaywidget))
    (:`else`)))

(fn `SGK HoldableMesh`
  (returns (Mesh :type "PrimitiveComponent Object Reference"))
  (`parent.SGK HoldableMesh`)
  (return (`self.StaticMesh`)))

(fn `ToggleBuildMenu`
  (params (Open :type Boolean))
  (locals (PlayerBuildingComponentL :type "/Game/SurvivalGameKitV2/Components/BP_PlayerBuildingComponent Object Reference"))
  ;[1 1 1] Open/close building menu
  (bind _playerinventory (`self.PlayerInventory`)
    (:`then`
      (bind _returnvalue (`self.GetComponentByClass` (`Pawn.GetController` (`/Game/SurvivalGameKitV2/Components/BP_PlayerInventory.SGKCharacter` _playerinventory)) "/Game/SurvivalGameKitV2/Components/BP_PlayerBuildingComponent.BP_PlayerBuildingComponent_C"))
      (`/Engine/EditorBlueprintResources/StandardMacros.IsValid` _returnvalue
        (:`Is Valid`
          (set `local.PlayerBuildingComponentL` _returnvalue)
          (if (`local.Open`)
            (bind _playerinventory_2 (`self.PlayerInventory`)
              (:`then`
                (if (not (`/Game/SurvivalGameKitV2/Components/BP_PlayerInventory.InventoryOpen` _playerinventory_2))
                  (`/Game/SurvivalGameKitV2/Components/BP_PlayerBuildingComponent.ToggleBuildOptionsMenu` (`local.PlayerBuildingComponentL`) true)))
              (:`else`))
            (else
              (bind _playerinventory_3 (`self.PlayerInventory`)
                (:`then`
                  (if (not (`/Game/SurvivalGameKitV2/Components/BP_PlayerInventory.InventoryOpen` _playerinventory_3))
                    (`/Game/SurvivalGameKitV2/Components/BP_PlayerBuildingComponent.ToggleBuildOptionsMenu` (`local.PlayerBuildingComponentL`) false)))
                (:`else`)))))))
    (:`else`)))

(fn `UserConstructionScript`
  (`parent.UserConstructionScript`))